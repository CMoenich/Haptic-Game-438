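; World-space callout label: an arrowhead, line and styled text widget that turn to face the player camera.
; The construction script chains the parts by mesh sockets, sizes them and previews yaw, while TextBoxProperties applies widget style and arrow colour through dynamic materials.
; Timeline updates drive the facing.
; With distance activation on, the callout starts hidden, then scales up when the camera comes within range and reverses when it leaves.
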(event EventBeginPlay
  (bind _returnvalue (Game|GetPlayerCameraManager 0))
  (bind _returnvalue_2 (Game|GetPlayerCameraManager 0))
  (bind _returnvalue_3 (Game|GetPlayerCameraManager 0))
  (bind _returnvalue_4 (Game|GetPlayerCameraManager 0))
  (bind _returnvalue_5 (Game|GetPlayerCameraManager 0))
  (bind _returnvalue_6 (Game|GetPlayerCameraManager 0))
  (bind _arrowhead_sm (Variables|Default|GetArrowHead_SM))
  (bind _arrowhead_sm_2 (Variables|Default|GetArrowHead_SM))
  (bind _arrowhead_sm_3 (Variables|Default|GetArrowHead_SM))
  (bind _arrowhead_sm_4 (Variables|Default|GetArrowHead_SM))
  (bind _widgetparent (Variables|Default|GetWidgetParent))
  (bind _arrowhead_sm_5 (Variables|Default|GetArrowHead_SM))
  (bind _widgetparent_2 (Variables|Default|GetWidgetParent))
  (bind _returnvalue_7 (Transformation|GetWorldLocation _arrowhead_sm_5))
  (bind _returnvalue_8 (Transformation|GetSocketLocation _arrowhead_sm_2 "Socket"))
  (bind _returnvalue_9 (Transformation|GetSocketLocation _widgetparent_2 "Socket"))
  (bind _returnvalue_10 (Transformation|GetSocketLocation _arrowhead_sm "None"))
  (bind _transformcomponent (Variables|/Script/Engine.PlayerCameraManager|GetTransformComponent _returnvalue_6))
  (bind _transformcomponent_2 (Variables|/Script/Engine.PlayerCameraManager|GetTransformComponent _returnvalue_2))
  (bind _transformcomponent_3 (Variables|/Script/Engine.PlayerCameraManager|GetTransformComponent _returnvalue_3))
  (bind _transformcomponent_4 (Variables|/Script/Engine.PlayerCameraManager|GetTransformComponent _returnvalue_4))
  (bind _transformcomponent_5 (Variables|/Script/Engine.PlayerCameraManager|GetTransformComponent _returnvalue_5))
  (bind _transformcomponent_6 (Variables|/Script/Engine.PlayerCameraManager|GetTransformComponent _returnvalue))
  (bind _returnvalue_11 (Transformation|GetWorldLocation _transformcomponent_6))
  (bind _returnvalue_12 (Transformation|GetWorldLocation _transformcomponent_2))
  (bind _returnvalue_13 (Transformation|GetWorldLocation _transformcomponent_3))
  (bind _returnvalue_14 (Transformation|GetWorldLocation _transformcomponent_4))
  (bind _returnvalue_15 (Transformation|GetWorldLocation _transformcomponent_5))
  (bind _returnvalue_16 (Transformation|GetWorldLocation _transformcomponent))
  (bind _returnvalue_17 (Math|Rotator|FindLookatRotation _returnvalue_8 _returnvalue_11))
  (bind _returnvalue_18 (Math|Vector|Distance(Vector) _returnvalue_16 _returnvalue_7))
  (bind _returnvalue_19 (Math|Rotator|FindLookatRotation _returnvalue_9 _returnvalue_12))
  (bind _returnvalue_20 (Math|Rotator|FindLookatRotation _returnvalue_8 _returnvalue_13))
  (bind _returnvalue_21 (Math|Rotator|FindLookatRotation _returnvalue_10 _returnvalue_14))
  (bind _returnvalue_22 (Math|Rotator|FindLookatRotation _returnvalue_10 _returnvalue_15))
  (Class|WidgetComponent|SetTwoSided (Variables|Default|GetWidgetParent) false)
  (Components|Timeline|SetPlayRate (Variables|Default|GetTimeline2) 0.75)
  (CallFunction|TextBoxProperties)
  (if (Variables|Default|GetActivate%20Based%20on%20Distance%20from%20Camera)
    (Development|SetHiddeninGame (Variables|Default|GetDefaultSceneRoot) true true)
    (Utilities|FlowControl|Delay 0.1)
    (Timeline|Timeline Play
      (:Update
        (if (Variables|Debug|GetDebug%20Distance)
          (Development|PrintString (Utilities|String|ToString(Float) _returnvalue_18)))
        (if (< _returnvalue_18 (Variables|Default|GetDistance%20to%20activate%20%28meters%29))
          (Development|SetHiddeninGame (Variables|Default|GetDefaultSceneRoot) false true)
          (bind _newtrack_0 (Timeline|Timeline2 Play)
            (:Update
              (Transformation|SetWorldScale3D _arrowhead_sm_4 (Math|Vector|MakeVector 1.0 (Math|Float|Lerp 0.0 (Variables|Default|GetArrow%20Head%20thickness) _newtrack_0) (Math|Float|Lerp 0.0 (Variables|ArrowProperties|GetArrow%20Head%20Length) _newtrack_0)))
              (Transformation|SetWorldLocation (Variables|Default|GetArrowLine_SM) (Transformation|GetSocketLocation _arrowhead_sm_4 "Socket") false false)
              (Transformation|SetWorldScale3D (Variables|Default|GetArrowLine_SM) (Math|Vector|MakeVector 1.0 (Math|Float|Lerp 0.0 (Variables|ArrowProperties|GetArrow%20Thickness_max) _newtrack_0) (Math|Float|Lerp 0.0 (Variables|ArrowProperties|GetArrow%20Length_max) _newtrack_0)))
              (Transformation|SetWorldScale3D (Variables|Default|GetWidgetParent) (Math|Conversions|ToVector(Float) (Math|Float|Lerp 0.0 (Variables|TextProperties|GetFont%20Size) _newtrack_0)))
              (Transformation|SetWorldLocation (Variables|Default|GetWidgetParent) (Transformation|GetSocketLocation (Variables|Default|GetArrowLine_SM) "Socket") false false)
              (Transformation|SetWorldRotation _widgetparent (Math|Rotator|FindLookatRotation (Transformation|GetSocketLocation _widgetparent "Socket") (Transformation|GetWorldLocation (Variables|/Script/Engine.PlayerCameraManager|GetTransformComponent (Game|GetPlayerCameraManager 0)))) false false)
              (Transformation|SetRelativeRotation (Variables|Default|GetArrowLine_SM) (Math|Rotator|MakeRotator 0.0 (.pitch _returnvalue_21) (.yaw _returnvalue_21)) false false)
              (Transformation|SetRelativeRotation _arrowhead_sm (Math|Rotator|MakeRotator 0.0 (.pitch _returnvalue_22) (.yaw _returnvalue_22)) false false)))
          (else
            (Timeline|Timeline2 Reverse)))))
    (else
      (Timeline|Timeline3 Play
        (:Update
          (Transformation|SetWorldScale3D _arrowhead_sm_3 (Math|Vector|MakeVector 0.0 (Variables|Default|GetArrow%20Head%20thickness) (Variables|ArrowProperties|GetArrow%20Head%20Length)))
          (Transformation|SetWorldLocation (Variables|Default|GetArrowLine_SM) (Transformation|GetSocketLocation _arrowhead_sm_3 "Socket") false false)
          (Transformation|SetWorldScale3D (Variables|Default|GetArrowLine_SM) (Math|Vector|MakeVector 0.0 (Variables|ArrowProperties|GetArrow%20Thickness_max) (Variables|ArrowProperties|GetArrow%20Length_max)))
          (Transformation|SetWorldScale3D (Variables|Default|GetWidgetParent) (Math|Conversions|ToVector(Float) (Variables|TextProperties|GetFont%20Size)))
          (Transformation|SetWorldLocation (Variables|Default|GetWidgetParent) (Transformation|GetSocketLocation (Variables|Default|GetArrowLine_SM) "Socket") false false)
          (Transformation|SetWorldRotation _widgetparent_2 (Math|Rotator|MakeRotator 0.0 (.pitch _returnvalue_19) (.yaw _returnvalue_19)) false false)
          (Transformation|SetRelativeRotation (Variables|Default|GetArrowLine_SM) (Math|Rotator|MakeRotator 0.0 (.pitch _returnvalue_20) (.yaw _returnvalue_20)) false false)
          (Transformation|SetRelativeRotation _arrowhead_sm_2 (Math|Rotator|MakeRotator 0.0 (.pitch _returnvalue_17) (.yaw _returnvalue_17)) false false))))))

(fn ConstructionScript
  (bind _widgetparent (Variables|Default|GetWidgetParent))
  (bind _arrowline_sm (Variables|Default|GetArrowLine_SM))
  (Transformation|SetWorldScale3D (Variables|Default|GetArrowHead_SM) (Math|Vector|MakeVector 0.0 (Variables|ArrowProperties|GetArrow%20Head%20Thickness) (Variables|ArrowProperties|GetArrow%20Head%20Length)))
  (Transformation|SetWorldLocation (Variables|Default|GetArrowLine_SM) (Transformation|GetSocketLocation (Variables|Default|GetArrowHead_SM) "Socket") false false)
  (Transformation|SetWorldScale3D _arrowline_sm (Math|Vector|MakeVector 1.0 (Variables|ArrowProperties|GetLine%20Thickness) (Variables|ArrowProperties|GetLine%20Length)))
  (Transformation|SetWorldLocation (Variables|Default|GetWidgetParent) (Transformation|GetSocketLocation _arrowline_sm "Socket") false false)
  (Rendering|SetCastShadow _widgetparent false)
  (Transformation|SetWorldScale3D _widgetparent (Math|Conversions|ToVector(Float) (Variables|TextProperties|GetFont%20Size)))
  (Variables|ArrowProperties|SetArrow%20Length_max (Variables|ArrowProperties|GetLine%20Length))
  (Variables|ArrowProperties|SetArrow%20Thickness_max (Variables|ArrowProperties|GetLine%20Thickness))
  (Transformation|SetRelativeRotation (Variables|Default|GetArrowHead_SM) (Math|Rotator|MakeRotator 0.0 0.0 (Math|Float|MapRangeClamped (Variables|Debug|GetPreview%20Rotation) 0.0 1.0 0.0 3.6e+02)) false false)
  (CallFunction|TextBoxProperties))

(fn TextBoxProperties
  (bind _widgetparent (Variables|Default|GetWidgetParent))
  (Default|UpdateWidget (Variables|Default|GetWidgetParent) (Variables|TextProperties|GetText) (Variables|TextProperties|GetFont%20Colour) (Variables|TextProperties|GetFont%20Style) (Variables|TextBoxProperties|GetPadding) (Variables|TextBoxProperties|GetTextbox%20Style) (Variables|TextBoxProperties|GetTextbox%20Corner%20Radius) (Variables|TextBoxProperties|GetTextbox%20Background%20Color) (Variables|TextBoxProperties|GetTextbox%20Outline%20Color) (Variables|TextBoxProperties|GetTextbox%20Outline%20Thickness))
  (Transformation|SetWorldRotation _widgetparent (Math|Rotator|MakeRotator 0.0 0.0 (.yaw (Transformation|GetWorldRotation _widgetparent))) false false)
  (bind _returnvalue (Rendering|Material|CreateDynamicMaterialInstance (Variables|Default|GetArrowHead_SM) 0 "/Game/TextBox/Materials/Arrow_Colour_M.Arrow_Colour_M" "None" :!class /Script/Engine.PrimitiveComponent))
  (Rendering|Material|SetVectorParameterValue _returnvalue "Colour" (Variables|ArrowProperties|GetArrow%20Colour) :!class /Script/Engine.MaterialInstanceDynamic)
  (bind _returnvalue_2 (Rendering|Material|CreateDynamicMaterialInstance (Variables|Default|GetArrowLine_SM) 0 "/Game/TextBox/Materials/Arrow_Colour_M.Arrow_Colour_M" "None" :!class /Script/Engine.PrimitiveComponent))
  (Rendering|Material|SetVectorParameterValue _returnvalue_2 "Colour" (Variables|ArrowProperties|GetArrow%20Colour) :!class /Script/Engine.MaterialInstanceDynamic))